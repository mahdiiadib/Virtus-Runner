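; Endless-runner track tile that fills its three lanes with random obstacles and pickups on BeginPlay.
; SpawnObstacle re-rolls at every nested range check, so lanes can stay empty; BoxCount limits only the right lane's box branch.
; Most right-lane spawns have no class set.
; When the player overlaps Box, it requests the next tile from the game mode, adds points, raises clamped walk speed, then destroys itself after a delay.
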(event `self.ReceiveBeginPlay`
  (`self.SpawnObstacle`))

(event `self.Box.OnComponentBeginOverlap`
  (params (OverlappedComponent :type "PrimitiveComponent Object Reference") (OtherActor :type "Actor Object Reference") (OtherComp :type "PrimitiveComponent Object Reference") (OtherBodyIndex :type Integer) (bFromSweep :type Boolean) (SweepResult :type "HitResult Structure (by ref)"))
  (cast `/Game/ThirdPersonBP/Blueprints/ThirdPersonCharacter` OtherActor)
  (bind _asthird_person_game_mode (cast `/Game/ThirdPersonBP/Blueprints/ThirdPersonGameMode` (`GameplayStatics.GetGameMode`)))
  (`/Game/ThirdPersonBP/Blueprints/ThirdPersonGameMode.SpawnTile` _asthird_person_game_mode)
  (set `/Game/ThirdPersonBP/Blueprints/ThirdPersonGameMode.CurrentPoints` (+ (`/Game/ThirdPersonBP/Blueprints/ThirdPersonGameMode.CurrentPoints` _asthird_person_game_mode) (* (`/Game/ThirdPersonBP/Blueprints/ThirdPersonGameMode.PointsMultiplier` _asthird_person_game_mode) 1)) _asthird_person_game_mode)
  (bind _asthird_person_character (cast `/Game/ThirdPersonBP/Blueprints/ThirdPersonCharacter` (`GameplayStatics.GetPlayerCharacter` 0)))
  (bind _charactermovement (`Character.CharacterMovement` _asthird_person_character))
  (set `CharacterMovementComponent.MaxWalkSpeed` (`KismetMathLibrary.FClamp` (* (`CharacterMovementComponent.MaxWalkSpeed` _charactermovement) 1.01) 800.0 1600.0) _charactermovement)
  (`KismetSystemLibrary.Delay` 10.0)
  (`self.K2_DestroyActor`))

(fn `SpawnObstacle`
  (locals (BoxCount :type Integer))
  (bind _returnvalue (`KismetMathLibrary.RandomFloatInRange` 0.0 1.0))
  (bind _returnvalue_2 (`KismetMathLibrary.RandomFloatInRange` 0.0 1.0))
  (bind _returnvalue_3 (`KismetMathLibrary.RandomFloatInRange` 0.0 1.0))
  (bind _returnvalue_4 (`SceneComponent.K2_GetComponentToWorld` (`self.LaneL`)))
  (bind _returnvalue_5 (`SceneComponent.K2_GetComponentToWorld` (`self.LaneR`)))
  (bind _returnvalue_6 (`SceneComponent.K2_GetComponentToWorld` (`self.LaneM`)))
  (`|ExecutionSequence`
    (:`then_0`
      ;[1 1 1] Lane Left
      (if (`KismetMathLibrary.InRange_FloatFloat` _returnvalue_2 0.0 0.2)
        (`|SpawnActorFromClass` "/Game/RunnerFiles/Blueprints/BP_ObstaclePipe_high.BP_ObstaclePipe_high_C" _returnvalue_4 "Undefined" "OverrideRootScale" null null)
        (elif (`KismetMathLibrary.InRange_FloatFloat` _returnvalue_2 0.2 0.4 false)
          (`|SpawnActorFromClass` "/Game/RunnerFiles/Blueprints/BP_ObstaclePipe.BP_ObstaclePipe_C" _returnvalue_4 "Undefined" "OverrideRootScale" null null)
          (elif (`KismetMathLibrary.InRange_FloatFloat` _returnvalue_2 0.4 0.5 false)
            (`|SpawnActorFromClass` "/Game/RunnerFiles/Blueprints/BP_ObstacleBox.BP_ObstacleBox_C" _returnvalue_4 "Undefined" "OverrideRootScale" null null)
            (`/Engine/EditorBlueprintResources/StandardMacros.IncrementInt` (`local.BoxCount`))
            (elif (`KismetMathLibrary.InRange_FloatFloat` _returnvalue_2 0.5 0.9 false)
              (`|SpawnActorFromClass` "/Game/RunnerFiles/Blueprints/BP_CoinPickup.BP_CoinPickup_C" _returnvalue_4 "Undefined" "OverrideRootScale" null null)
              (elif (`KismetMathLibrary.InRange_FloatFloat` _returnvalue_2 0.9 0.95 false)
                (`|SpawnActorFromClass` "/Game/RunnerFiles/Blueprints/BP_MagnetPickup.BP_MagnetPickup_C" _returnvalue_4 "Undefined" "OverrideRootScale" null null)
                (elif (`KismetMathLibrary.InRange_FloatFloat` _returnvalue_2 0.95 1.0 false)
                  (`|SpawnActorFromClass` "/Game/RunnerFiles/Blueprints/BP_BootsPickup.BP_BootsPickup_C" _returnvalue_4 "Undefined" "OverrideRootScale" null null))))))))
    (:`then_1`
      ;[1 1 1] Lane Middle
      (if (`KismetMathLibrary.InRange_FloatFloat` _returnvalue_3 0.0 0.2)
        (`|SpawnActorFromClass` "/Game/RunnerFiles/Blueprints/BP_ObstaclePipe_high.BP_ObstaclePipe_high_C" _returnvalue_6 "Undefined" "OverrideRootScale" null null)
        (elif (`KismetMathLibrary.InRange_FloatFloat` _returnvalue_3 0.2 0.4 false)
          (`|SpawnActorFromClass` "/Game/RunnerFiles/Blueprints/BP_ObstaclePipe.BP_ObstaclePipe_C" _returnvalue_6 "Undefined" "OverrideRootScale" null null)
          (elif (`KismetMathLibrary.InRange_FloatFloat` _returnvalue_3 0.4 0.5 false)
            (`|SpawnActorFromClass` "/Game/RunnerFiles/Blueprints/BP_ObstacleBox.BP_ObstacleBox_C" _returnvalue_6 "Undefined" "OverrideRootScale" null null)
            (`/Engine/EditorBlueprintResources/StandardMacros.IncrementInt` (`local.BoxCount`))
            (elif (`KismetMathLibrary.InRange_FloatFloat` _returnvalue_3 0.5 0.9 false)
              (`|SpawnActorFromClass` "/Game/RunnerFiles/Blueprints/BP_CoinPickup.BP_CoinPickup_C" _returnvalue_6 "Undefined" "OverrideRootScale" null null)
              (elif (`KismetMathLibrary.InRange_FloatFloat` _returnvalue_3 0.9 0.95 false)
                (`|SpawnActorFromClass` "/Game/RunnerFiles/Blueprints/BP_MagnetPickup.BP_MagnetPickup_C" _returnvalue_6 "Undefined" "OverrideRootScale" null null)
                (elif (`KismetMathLibrary.InRange_FloatFloat` _returnvalue_3 0.95 1.0 false)
                  (`|SpawnActorFromClass` "/Game/RunnerFiles/Blueprints/BP_BootsPickup.BP_BootsPickup_C" _returnvalue_6 "Undefined" "OverrideRootScale" null null))))))))
    (:`then_2`
      ;[1 1 1] Lane Right
      (if (`KismetMathLibrary.InRange_FloatFloat` _returnvalue 0.0 0.2)
        (`|SpawnActorFromClass` "/Game/RunnerFiles/Blueprints/BP_ObstaclePipe_high.BP_ObstaclePipe_high_C" _returnvalue_5 "Undefined" "OverrideRootScale" null null)
        (elif (`KismetMathLibrary.InRange_FloatFloat` _returnvalue 0.2 0.4 false)
          (`|SpawnActorFromClass` "/Game/RunnerFiles/Blueprints/BP_ObstaclePipe.BP_ObstaclePipe_C" _returnvalue_5 "Undefined" "OverrideRootScale" null null)
          (elif (`KismetMathLibrary.InRange_FloatFloat` _returnvalue 0.4 0.5 false)
            (if (< (`local.BoxCount`) 2)
              (`|SpawnActorFromClass` "/Game/RunnerFiles/Blueprints/BP_ObstacleBox.BP_ObstacleBox_C" _returnvalue_5 "Undefined" "OverrideRootScale" null null)
              (`/Engine/EditorBlueprintResources/StandardMacros.IncrementInt` (`local.BoxCount`)))
            (elif (`KismetMathLibrary.InRange_FloatFloat` _returnvalue 0.5 0.9 false)
              (`|SpawnActorFromClass` "/Game/RunnerFiles/Blueprints/BP_CoinPickup.BP_CoinPickup_C" _returnvalue_5 "Undefined" "OverrideRootScale" null null)
              (elif (`KismetMathLibrary.InRange_FloatFloat` _returnvalue 0.9 0.95 false)
                (`|SpawnActorFromClass` "/Game/RunnerFiles/Blueprints/BP_MagnetPickup.BP_MagnetPickup_C" _returnvalue_5 "Undefined" "OverrideRootScale" null null)
                (elif (`KismetMathLibrary.InRange_FloatFloat` _returnvalue 0.95 1.0 false)
                  (`|SpawnActorFromClass` "/Game/RunnerFiles/Blueprints/BP_BootsPickup.BP_BootsPickup_C" _returnvalue_5 "Undefined" "OverrideRootScale" null null))))))))))

(fn `UserConstructionScript`)